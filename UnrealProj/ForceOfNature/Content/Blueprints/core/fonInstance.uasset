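; Game instance Blueprint that serves as a central hub for launching prototype maps and showing the game's menus.
; Two play events open the disaster test level and the world map by name.
; Main, options, language and debug level-select events each create their widget on first use, cache it and add it to the viewport.
; Only the main menu event also enables the mouse cursor.
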(event `PlayDisasterPrototype`
  ;[1 1 1] Start a singleplayer Map
  (`GameplayStatics.OpenLevel` "levelTest"))

(event `PlayWorldMapPrototype`
  ;[1 1 1] Start a singleplayer Map
  (`GameplayStatics.OpenLevel` "worldMap"))

(event `ShowMainMenu`
  (bind _returnvalue (`GameplayStatics.GetPlayerController` 0))
  ;[1 1 1] Show Main Menu
  (`/Engine/EditorBlueprintResources/StandardMacros.IsValid` (`self.mainMenuWidget`)
    (:`Is Valid`
      _)
    (:`Is Not Valid`
      (bind _returnvalue_2 (`|CreateWidget` "/Game/Blueprints/gui/Menus/MainMenuWidget.MainMenuWidget_C" _returnvalue))
      (set `self.mainMenuWidget` _returnvalue_2)))
  (`UserWidget.AddToViewport` (`self.mainMenuWidget`) 0)
  (set `PlayerController.bShowMouseCursor` true _returnvalue))

(event `ShowOptionsMenu`
  ;[1 1 1] Show Options Menu
  (`/Engine/EditorBlueprintResources/StandardMacros.IsValid` (`self.optionsWidget`)
    (:`Is Valid`
      _)
    (:`Is Not Valid`
      (bind _returnvalue (`|CreateWidget` "/Game/Blueprints/gui/Menus/OptionsMenu.OptionsMenu_C" (`GameplayStatics.GetPlayerController` 0)))
      (set `self.optionsWidget` _returnvalue)))
  (`UserWidget.AddToViewport` (`self.optionsWidget`) 0))

(event `ShowLanguageMenu`
  ;[1 1 1] Show Language Menu
  (`/Engine/EditorBlueprintResources/StandardMacros.IsValid` (`self.languageWidget`)
    (:`Is Valid`
      _)
    (:`Is Not Valid`
      (bind _returnvalue (`|CreateWidget` "/Game/Blueprints/gui/Menus/LanguageMenu.LanguageMenu_C" (`GameplayStatics.GetPlayerController` 0)))
      (set `self.languageWidget` _returnvalue)))
  (`UserWidget.AddToViewport` (`self.languageWidget`) 0))

(event `ShowDebugLevelSelect`
  ;[1 1 1] Show ShowDebugLevelSelect Menu
  (`/Engine/EditorBlueprintResources/StandardMacros.IsValid` (`self.debugLevelSelectWidget`)
    (:`Is Valid`
      _)
    (:`Is Not Valid`
      (bind _returnvalue (`|CreateWidget` "/Game/Blueprints/gui/Menus/DebugLevelSelectMenu.DebugLevelSelectMenu_C" (`GameplayStatics.GetPlayerController` 0)))
      (set `self.debugLevelSelectWidget` _returnvalue)))
  (`UserWidget.AddToViewport` (`self.debugLevelSelectWidget`) 0))