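; A clickable path node for the disaster levels, linked to up to four neighboring nodes in the left, right, up and down directions.
; On BeginPlay it caches the levelGM game mode and gathers its assigned neighbors into a single list for connection checks and group highlighting.
; Clicking the platform reports the node to the game mode, and highlighting swaps the platform's material.
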(event `self.ReceiveBeginPlay`
  (`self.GetReferences`)
  (`self.MakeConnectedIntoList`))

(event `self.Platform.OnClicked`
  (params (TouchedComponent :type "PrimitiveComponent Object Reference") (ButtonPressed :type "Key Structure"))
  (`/Game/Blueprints/disasterLevels/player/levelGM.ClickedNode` (`self.gameMode`) self))

(fn `GetReferences`
  (bind _aslevel_gm (cast `/Game/Blueprints/disasterLevels/player/levelGM` (`GameplayStatics.GetGameMode`))
    (:`then`
      (set `self.gameMode` _aslevel_gm))
    (:`CastFailed`
      (`/Game/Blueprints/libraries/fonLib.PrintError` "pathNode getreferences cast to levelGM failed"))))

(fn `HighlightConnected`
  (params (highlight :type Boolean))
  (locals (current :type "/Game/Blueprints/disasterLevels/pathNode Object Reference"))
  ;[1 0 0] For Loop
  (for _array_element (`self.allConnected`)
    (`self.SetHighlighted` _array_element highlight)))

(fn `IsConnectedTo`
  (params (other :type "/Game/Blueprints/disasterLevels/pathNode Object Reference"))
  (returns (connected :type Boolean))
  (return (`KismetArrayLibrary.Array_Contains` (`self.allConnected`) other)))

(fn `MakeConnectedIntoList`
  (locals (current :type "/Game/Blueprints/disasterLevels/pathNode Object Reference"))
  (`|ExecutionSequence`
    (:`then_0`
      (set `local.current` (`self.leftConnected`)))
    (:`then_1`
      (set `local.current` (`self.rightConnected`)))
    (:`then_2`
      (set `local.current` (`self.upConnected`)))
    (:`then_3`
      (set `local.current` (`self.downConnected`))))
  (if (!= (`local.current`) null)
    (`KismetArrayLibrary.Array_Add` (`self.allConnected`) (`local.current`))))

(fn `SetHighlighted`
  (params (highlighted :type Boolean))
  (locals (matToSet :type "MaterialInterface Object Reference"))
  (if highlighted
    (set `local.matToSet` (`self.highlightMat`))
    (else
      (set `local.matToSet` (`self.defaultMat`))))
  (`PrimitiveComponent.SetMaterial` (`self.Platform`) 0 (`local.matToSet`)))

(fn `UserConstructionScript`)