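; fonDataLib is a function library that looks up textures by name for disaster icons and quest givers.
; GetDisasterIconByName switches on the name to return a flame, tornado, fissure or rocks icon, with AICONGreen as the fallback.
; GetQuestGiverByName does the same for quest givers, knowing only Person and falling back to MaterialError for any other name.
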(fn `GetDisasterIconByName`
  (params (name :type String))
  (returns (texture :type "Texture2D Object Reference"))
  (locals (textureToReturn :type "Texture2D Object Reference" :default null))
  (`|ExecutionSequence`
    (:`then_0`
      (switch `string` name
        (:`Default`
          (set `local.textureToReturn` "/Engine/EngineResources/AICON-Green.AICON-Green"))
        (:`flame`
          (set `local.textureToReturn` "/Game/TEMPORARY/art-assets/quiz/possibleAnswerIcons/flame.flame"))
        (:`tornado`
          (set `local.textureToReturn` "/Game/TEMPORARY/art-assets/quiz/possibleAnswerIcons/tornado.tornado"))
        (:`fissure`
          (set `local.textureToReturn` "/Game/TEMPORARY/art-assets/quiz/possibleAnswerIcons/fissure.fissure"))
        (:`rocks`
          (set `local.textureToReturn` "/Game/TEMPORARY/art-assets/quiz/possibleAnswerIcons/rocks.rocks"))))
    (:`then_1`
      (return (`local.textureToReturn`)))))

(fn `GetQuestGiverByName`
  (params (name :type String))
  (returns (texture :type "Texture2D Object Reference"))
  (locals (textureToReturn :type "Texture2D Object Reference"))
  (`|ExecutionSequence`
    (:`then_0`
      (switch `string` name
        (:`Default`
          (set `local.textureToReturn` "/Engine/EngineDebugMaterials/MaterialError.MaterialError"))
        (:`person`
          (set `local.textureToReturn` "/Game/TEMPORARY/art-assets/quiz/questGivers/person.person"))))
    (:`then_1`
      (return (`local.textureToReturn`)))))