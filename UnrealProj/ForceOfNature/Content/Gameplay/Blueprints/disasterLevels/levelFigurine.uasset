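; Base Blueprint for a figurine that occupies and moves between nodes in a level.
; On init it stores the GameMode and registers with its starting node as an occupant.
; SetPosition notifies the old node, records it in PathHistory and enters the new node, which now handles the actor's placement.
; ExecuteMoveAction and FigurineSteppedOnMyNode are empty hooks for child Blueprints to override.
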(fn `ExecuteMoveAction`
  ;[1 1 1] OVERWRITE IN CHILD BPs!
)

(fn `FigurineSteppedOnMyNode`
  (params (otherFigurine :type "/Game/Gameplay/Blueprints/disasterLevels/levelFigurine Object Reference"))
  ;[1 1 1] override by children, for those that do anything with this.
)

(fn `InitFigurine`
  (params (gameMode :type "/Game/Gameplay/Blueprints/disasterLevels/player/levelGM Object Reference"))
  (set `self.gameMode` gameMode)
  (`self.SetInitialPosition` (`self.startingNode`)))

(fn `SetInitialPosition`
  (params (node :type "/Game/Gameplay/Blueprints/disasterLevels/pathNode Object Reference"))
  (bind _output_get (set `self.currentNode` node))
  (`/Game/Gameplay/Blueprints/disasterLevels/pathNode.AddStartingOccupant` _output_get self)
  (`/Game/Gameplay/Blueprints/disasterLevels/pathNode.EnterNodeInit` _output_get self))

(fn `SetPosition`
  (params (node :type "/Game/Gameplay/Blueprints/disasterLevels/pathNode Object Reference"))
  (`/Game/Gameplay/Blueprints/disasterLevels/pathNode.IsSteppedOff` (`self.currentNode`) self)
  (`KismetArrayLibrary.Array_Add` (`self.pathHistory`) (`self.currentNode`))
  (set `self.currentNode` node)
  (`/Game/Gameplay/Blueprints/disasterLevels/pathNode.EnterNode` node self))

(fn `UserConstructionScript`)