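; Level exit node Blueprint for the disaster levels that signals when the player's figurine reaches the exit.
; It extends a parent node's IsSteppedon event, calling the parent before running its own check.
; If the stepper matches the GameMode's PlayerFigurine, it tells the GameMode that the player reached the exit node.
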(event `self.IsSteppedOn`
  (params (stepper :type "/Game/Gameplay/Blueprints/disasterLevels/levelFigurine Object Reference"))
  (`parent.IsSteppedOn` stepper)
  (`self.LevelExitNodeIsSteppedOn` stepper))

(fn `LevelExitNodeIsSteppedOn`
  (params (Stepper :type "/Game/Gameplay/Blueprints/disasterLevels/levelFigurine Object Reference"))
  (if (== Stepper (`/Game/Gameplay/Blueprints/disasterLevels/player/levelGM.playerFigurine` (`self.gameMode`)))
    (`/Game/Gameplay/Blueprints/disasterLevels/player/levelGM.PlayerReachedExitNode` (`self.gameMode`))))

(fn `UserConstructionScript`
  (`parent.UserConstructionScript`))