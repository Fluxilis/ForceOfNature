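; Distribution box figurine for a node-based level, a hazard that is dangerous to the player from the side it faces.
; It overrides the figurine move prediction, move execution and stepped-on hooks, with both move functions left empty.
; When the player enters its node, it compares the player's last path-history node with the node in its look direction.
; A match only prints a death message.
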(event `self.PredictTypeSpecificNextMove`
  (`self.DistributionBoxPredictNextMove`))

(event `self.ExecuteTypeSpecificMove`
  (`self.DistributionBoxExecuteMove`))

(event `self.FigurineSteppedOnMyNode`
  (params (otherFigurine :type "/Game/Gameplay/Blueprints/disasterLevels/levelFigurine Object Reference"))
  (`self.DistributionBoxFigurineSteppedOnNode` otherFigurine))

(fn `DistributionBoxExecuteMove`)

(fn `DistributionBoxFigurineSteppedOnNode`
  (params (otherFigurine :type "/Game/Gameplay/Blueprints/disasterLevels/levelFigurine Object Reference"))
  (bind _playerfigurine (`/Game/Gameplay/Blueprints/disasterLevels/player/levelGM.playerFigurine` (`self.gameMode`)))
  (bind _pathhistory (`/Game/Gameplay/Blueprints/disasterLevels/levelFigurine.pathHistory` _playerfigurine))
  (if (== otherFigurine _playerfigurine)
    (if (== (`/Game/Gameplay/Blueprints/disasterLevels/pathNode.GetSideConnectedNode` (`self.currentNode`) (`self.GetLookDirection`)) (`|GetArrayItem` _pathhistory (- (`KismetArrayLibrary.Array_Length` _pathhistory) 1)))
      (`/Game/Gameplay/Blueprints/libraries/fonLib.PrintInfo` "PLAYER DEAD"))))

(fn `DistributionBoxPredictNextMove`)

(fn `UserConstructionScript`
  (`parent.UserConstructionScript`))