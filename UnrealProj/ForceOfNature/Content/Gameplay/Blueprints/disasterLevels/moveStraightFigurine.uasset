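; Figurine Blueprint for the disaster levels that patrols a node grid in a straight line, one step per ExecuteMove.
; It follows the current direction through the node's connected neighbours and reverses when that side has no connection.
; After each move it checks whether it shares the player's node, currently only printing a kill message.
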(event `self.ExecuteMove`
  (`self.StraighterExecuteMove`))

(fn `StraighterExecuteMove`
  (bind _nextgoal (`self.StraighterGetNextGoalNode`))
  (`self.SetPosition` _nextgoal)
  (bind _onplayernode (`self.IsOnPlayerNode`))
  (if _onplayernode
    (`/Game/Gameplay/Blueprints/libraries/fonLib.PrintInfo` "Killed player!")))

(fn `StraighterGetNextGoalNode`
  (returns (nextGoal :type "/Game/Gameplay/Blueprints/disasterLevels/pathNode Object Reference"))
  (locals (nextTargetNode :type "/Game/Gameplay/Blueprints/disasterLevels/pathNode Object Reference"))
  (bind _leftconnected (`/Game/Gameplay/Blueprints/disasterLevels/pathNode.leftConnected` (`self.currentNode`)))
  (bind _upconnected (`/Game/Gameplay/Blueprints/disasterLevels/pathNode.upConnected` (`self.currentNode`)))
  (bind _downconnected (`/Game/Gameplay/Blueprints/disasterLevels/pathNode.downConnected` (`self.currentNode`)))
  (bind _leftconnected_2 (`/Game/Gameplay/Blueprints/disasterLevels/pathNode.leftConnected` (`self.currentNode`)))
  (bind _rightconnected (`/Game/Gameplay/Blueprints/disasterLevels/pathNode.rightConnected` (`self.currentNode`)))
  (bind _upconnected_2 (`/Game/Gameplay/Blueprints/disasterLevels/pathNode.upConnected` (`self.currentNode`)))
  (bind _rightconnected_2 (`/Game/Gameplay/Blueprints/disasterLevels/pathNode.rightConnected` (`self.currentNode`)))
  (bind _downconnected_2 (`/Game/Gameplay/Blueprints/disasterLevels/pathNode.downConnected` (`self.currentNode`)))
  (set `local.nextTargetNode` null) ; reset
  (`|ExecutionSequence`
    (:`then_0`
      (switch `/Game/Gameplay/Blueprints/libraries/direction` (`self.currentMoveDirection`)
        (:`NewEnumerator0`
          (`/Engine/EditorBlueprintResources/StandardMacros.IsValid` _upconnected
            (:`Is Valid`
              (set `local.nextTargetNode` _upconnected))
            (:`Is Not Valid`
              (`/Engine/EditorBlueprintResources/StandardMacros.IsValid` _downconnected_2
                (:`Is Valid`
                  (set `local.nextTargetNode` _downconnected_2)
                  (set `self.currentMoveDirection` "NewEnumerator2"))))))
        (:`NewEnumerator1`
          (`/Engine/EditorBlueprintResources/StandardMacros.IsValid` _rightconnected
            (:`Is Valid`
              (set `local.nextTargetNode` _rightconnected))
            (:`Is Not Valid`
              (`/Engine/EditorBlueprintResources/StandardMacros.IsValid` _leftconnected
                (:`Is Valid`
                  (set `local.nextTargetNode` _leftconnected)
                  (set `self.currentMoveDirection` "NewEnumerator3"))))))
        (:`NewEnumerator2`
          (`/Engine/EditorBlueprintResources/StandardMacros.IsValid` _downconnected
            (:`Is Valid`
              (set `local.nextTargetNode` _downconnected))
            (:`Is Not Valid`
              (`/Engine/EditorBlueprintResources/StandardMacros.IsValid` _upconnected_2
                (:`Is Valid`
                  (set `local.nextTargetNode` _upconnected_2)
                  (set `self.currentMoveDirection` "NewEnumerator0"))))))
        (:`NewEnumerator3`
          (`/Engine/EditorBlueprintResources/StandardMacros.IsValid` _leftconnected_2
            (:`Is Valid`
              (set `local.nextTargetNode` _leftconnected_2))
            (:`Is Not Valid`
              (`/Engine/EditorBlueprintResources/StandardMacros.IsValid` _rightconnected_2
                (:`Is Valid`
                  (set `local.nextTargetNode` _rightconnected_2)
                  (set `self.currentMoveDirection` "NewEnumerator1"))))))))
    (:`then_1`
      (return (`local.nextTargetNode`)))))

(fn `UserConstructionScript`
  (`parent.UserConstructionScript`))