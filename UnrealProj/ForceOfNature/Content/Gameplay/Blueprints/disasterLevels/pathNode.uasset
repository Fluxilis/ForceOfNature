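; Clickable board node in the disaster levels that figurines stand on, linked to up to four directional neighbours.
; On BeginPlay it resets its material, caches levelGM and gathers neighbours into a list for highlighting and connection checks.
; Platform clicks are forwarded to the game mode.
; Entering figurines snap to their numbered slot among five, and existing occupants are notified before the newcomer joins the occupant list.
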(event `self.ReceiveBeginPlay`
  (`self.Init`))

(event `self.Platform.OnClicked`
  (params (TouchedComponent :type "PrimitiveComponent Object Reference") (ButtonPressed :type "Key Structure"))
  (`self.ClickedInput`))

(fn `AddStartingOccupant`
  (params (figurine :type "/Game/Gameplay/Blueprints/disasterLevels/levelFigurine Object Reference (by ref)"))
  (`KismetArrayLibrary.Array_Add` (`self.currentOccupants`) figurine))

(fn `ClickedInput`
  (`/Game/Gameplay/Blueprints/disasterLevels/player/levelGM.ClickedNode` (`self.gameMode`) self))

(fn `EnterNode`
  (params (figurine :type "/Game/Gameplay/Blueprints/disasterLevels/levelFigurine Object Reference"))
  (locals (newSlotNr :type Integer))
  (`self.K2_SetActorLocation` figurine (`SceneComponent.K2_GetComponentLocation` (`self.GetSlot` (`/Game/Gameplay/Blueprints/disasterLevels/levelFigurine.nodeSlotNr` figurine))) false false)
  (`self.IsSteppedOn` figurine))

(fn `EnterNodeInit`
  (params (figurine :type "/Game/Gameplay/Blueprints/disasterLevels/levelFigurine Object Reference"))
  (`self.K2_SetActorLocation` figurine (`SceneComponent.K2_GetComponentLocation` (`self.GetSlot` (`/Game/Gameplay/Blueprints/disasterLevels/levelFigurine.nodeSlotNr` figurine))) false false))

(fn `GetReferences`
  (bind _aslevel_gm (cast `/Game/Gameplay/Blueprints/disasterLevels/player/levelGM` (`GameplayStatics.GetGameMode`))
    (:`then`
      (set `self.gameMode` _aslevel_gm))
    (:`CastFailed`
      (`/Game/Gameplay/Blueprints/libraries/fonLib.PrintError` "pathNode getreferences cast to levelGM failed"))))

(fn `GetSideConnectedNode`
  (params (direction :type "/Game/Gameplay/Blueprints/libraries/direction Enum" :default "NewEnumerator4"))
  (returns (connectedNode :type "/Game/Gameplay/Blueprints/disasterLevels/pathNode Object Reference"))
  (switch `/Game/Gameplay/Blueprints/libraries/direction` direction
    (:`NewEnumerator4`
      (`/Game/Gameplay/Blueprints/libraries/fonLib.PrintError` "pathNode GetConnectedNode no node can be connected in \"none\" direction!"))
    (:`NewEnumerator0`
      (return (`self.upConnected`)))
    (:`NewEnumerator1`
      (return (`self.rightConnected`)))
    (:`NewEnumerator2`
      (return (`self.downConnected`)))
    (:`NewEnumerator3`
      (return (`self.leftConnected`)))))

(fn `GetSlot`
  (params (slotNr :type Integer))
  (returns (slot :type "SceneComponent Object Reference"))
  (locals (slotToReturn :type "SceneComponent Object Reference"))
  (`|ExecutionSequence`
    (:`then_0`
      (switch `int` slotNr
        (:`Default`
          (`/Game/Gameplay/Blueprints/libraries/fonLib.PrintError` "pathNode GetSlot Error, no slot declared! (0 or >5)"))
        (:`1`
          (set `local.slotToReturn` (`self.slot1`)))
        (:`2`
          (set `local.slotToReturn` (`self.slot2`)))
        (:`3`
          (set `local.slotToReturn` (`self.slot3`)))
        (:`4`
          (set `local.slotToReturn` (`self.slot4`)))
        (:`5`
          (set `local.slotToReturn` (`self.slot5`)))))
    (:`then_1`
      (return (`local.slotToReturn`)))))

(fn `HighlightConnected`
  (params (highlight :type Boolean))
  (locals (current :type "/Game/Gameplay/Blueprints/disasterLevels/pathNode Object Reference"))
  ;[1 0 0] For Loop
  (for _array_element (`self.allConnected`)
    (`self.SetHighlighted` _array_element highlight)))

(fn `Init`
  ;[1 1 1] to set the initial material
  (`self.SetHighlighted` false)
  (`self.GetReferences`)
  (`self.MakeConnectedIntoList`))

(fn `IsConnectedTo`
  (params (other :type "/Game/Gameplay/Blueprints/disasterLevels/pathNode Object Reference"))
  (returns (connected :type Boolean))
  (return (`KismetArrayLibrary.Array_Contains` (`self.allConnected`) other)))

(fn `IsSteppedOff`
  (params (stepper :type "/Game/Gameplay/Blueprints/disasterLevels/levelFigurine Object Reference"))
  (bind _returnvalue (`KismetArrayLibrary.Array_RemoveItem` (`self.currentOccupants`) stepper))
  (if (not _returnvalue)
    (`/Game/Gameplay/Blueprints/libraries/fonLib.PrintError` "pathNode IsSteppedOff Tried to remove currentOccupant, but could not find in list of occupants!!")))

(fn `IsSteppedOn`
  (params (stepper :type "/Game/Gameplay/Blueprints/disasterLevels/levelFigurine Object Reference"))
  (`|ExecutionSequence`
    (:`then_0`
      ;[1 0 0] FOR LOOP
      (for _array_element (`self.currentOccupants`)
        (`/Game/Gameplay/Blueprints/disasterLevels/levelFigurine.FigurineSteppedOnMyNode` _array_element stepper)))
    (:`then_1`
      (`KismetArrayLibrary.Array_Add` (`self.currentOccupants`) stepper))))

(fn `MakeConnectedIntoList`
  (locals (current :type "/Game/Gameplay/Blueprints/disasterLevels/pathNode Object Reference"))
  (`|ExecutionSequence`
    (:`then_0`
      (set `local.current` (`self.leftConnected`)))
    (:`then_1`
      (set `local.current` (`self.rightConnected`)))
    (:`then_2`
      (set `local.current` (`self.upConnected`)))
    (:`then_3`
      (set `local.current` (`self.downConnected`))))
  (if (!= (`local.current`) null)
    (`KismetArrayLibrary.Array_Add` (`self.allConnected`) (`local.current`))))

(fn `SetHighlighted`
  (params (highlighted :type Boolean))
  (locals (matToSet :type "MaterialInterface Object Reference"))
  (if highlighted
    (set `local.matToSet` (`self.highlightMat`))
    (else
      (set `local.matToSet` (`self.defaultMat`))))
  (`PrimitiveComponent.SetMaterial` (`self.Platform`) 0 (`local.matToSet`)))

(fn `UserConstructionScript`)