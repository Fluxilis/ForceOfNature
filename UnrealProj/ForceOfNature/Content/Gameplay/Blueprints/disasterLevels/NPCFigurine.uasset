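; Base Blueprint for NPC figurines that move on a node-based board, with a look direction shown by an arrow.
; On init and after each move action it runs overridable execute and predict hooks, left empty here for specific NPC types, then refreshes the arrow.
; The arrow takes a preset relative transform per direction, and a helper checks whether the NPC shares its node with the player figurine.
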(event `self.ReceiveBeginPlay`
  (`parent.ReceiveBeginPlay`)
  (`self.UpdateLookDirectionArrow`))

(event `self.InitFigurine`
  (params (gameMode :type "/Game/Gameplay/Blueprints/disasterLevels/player/levelGM Object Reference"))
  (`parent.InitFigurine` gameMode)
  (`self.PredictTypeSpecificNextMove`)
  (`self.UpdateLookDirectionArrow`))

(event `self.ExecuteMoveAction`
  (`parent.ExecuteMoveAction`)
  (`self.ExecuteTypeSpecificMove`)
  (`self.PredictTypeSpecificNextMove`)
  (`self.UpdateLookDirectionArrow`))

(fn `ExecuteTypeSpecificMove`
  ;[1 1 1] OVERRIDE
)

(fn `GetLookDirection`
  (returns (currentLookDirection :type "/Game/Gameplay/Blueprints/libraries/direction Enum"))
  (return (`self.currentLookDirection`)))

(fn `IsOnPlayerNode`
  (returns (onPlayerNode :type Boolean))
  (return (`KismetArrayLibrary.Array_Contains` (`/Game/Gameplay/Blueprints/disasterLevels/pathNode.currentOccupants` (`self.currentNode`)) (`/Game/Gameplay/Blueprints/disasterLevels/player/levelGM.playerFigurine` (`self.gameMode`)))))

(fn `PredictTypeSpecificNextMove`)

(fn `SetLookDirection`
  (params (newLookDirection :type "/Game/Gameplay/Blueprints/libraries/direction Enum" :default "NewEnumerator4"))
  (set `self.currentLookDirection` newLookDirection)
  (`self.UpdateLookDirectionArrow`))

(fn `UpdateLookDirectionArrow`
  (locals (transformToSet :type "Transform Structure" :default "0.000000,0.000000,0.000000|0.000000,0.000000,-179.999954|1.250000,1.250000,0.555555"))
  (`|ExecutionSequence`
    (:`then_0`
      (switch `/Game/Gameplay/Blueprints/libraries/direction` (`self.currentLookDirection`)
        (:`NewEnumerator4`
          (set `local.transformToSet` (struct)))
        (:`NewEnumerator0`
          (set `local.transformToSet` (`self.daUp`)))
        (:`NewEnumerator1`
          (set `local.transformToSet` (`self.daRight`)))
        (:`NewEnumerator2`
          (set `local.transformToSet` (`self.daDown`)))
        (:`NewEnumerator3`
          (set `local.transformToSet` (`self.daLeft`)))))
    (:`then_1`
      (`SceneComponent.K2_SetRelativeTransform` (`self.directionArrow`) (`local.transformToSet`) false false))))

(fn `UserConstructionScript`
  (`parent.UserConstructionScript`))