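; GlobeWorldmap is the clickable globe actor on the world map, with a surface material localized to the current culture.
; On BeginPlay it picks the English or German material, logging an error and defaulting to English for unknown cultures, and caches the worldMapPC controller.
; Clicks and releases on the globe mesh are forwarded to that controller, with clicks passing the Winkel transform and the mesh.
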(event `self.GlobeMesh.OnClicked`
  (params (TouchedComponent :type "PrimitiveComponent Object Reference") (ButtonPressed :type "Key Structure"))
  (`/Game/Gameplay/Blueprints/worldMap/player/worldMapPC.GlobeClicked` (stale `self.ReceiveBeginPlay` _output_get) (`self.Winkel`) (`self.GlobeMesh`)))

(event `self.ReceiveBeginPlay`
  (`self.Localize`)
  (bind _asworld_map_pc (cast `/Game/Gameplay/Blueprints/worldMap/player/worldMapPC` (`GameplayStatics.GetPlayerController` 0))
    (:`then`
      (bind _output_get (set `self.PlayerControllerRef` _asworld_map_pc)))
    (:`CastFailed`
      (`/Game/Gameplay/Blueprints/libraries/fonLib.PrintError` "Couldn't cast PC to WorldMapPC in GlobeWorldmap"))))

(event `self.GlobeMesh.OnReleased`
  (params (TouchedComponent :type "PrimitiveComponent Object Reference") (ButtonReleased :type "Key Structure"))
  (`/Game/Gameplay/Blueprints/worldMap/player/worldMapPC.GlobeReleased` (stale `self.ReceiveBeginPlay` _output_get)))

(fn `Localize`
  (bind _returnvalue (`KismetInternationalizationLibrary.GetCurrentCulture`))
  (switch `string` _returnvalue
    (:`Default`
      (`/Game/Gameplay/Blueprints/libraries/fonLib.PrintError` (`KismetStringLibrary.Concat_StrStr` "GlobeWorldmap SetLoca error. Loca not found for: " _returnvalue " \nSet to default (english)."))
      (`PrimitiveComponent.SetMaterial` (`self.GlobeMesh`) 0 (`self.baseMaterial_en`) :!label _label))
    (:`en`
      (goto _label))
    (:`de-DE`
      (`PrimitiveComponent.SetMaterial` (`self.GlobeMesh`) 0 (`self.baseMaterial_de-DE`)))))

(fn `UserConstructionScript`)