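; Game instance that handles level flow, language and shared menus for a disaster-event game with a world map.
; Disaster events start from a quiz and step through up to ten levels read from a DataTable row, returning to the world map when the next entry is None.
; Helpers restart levels, reset per-level data and set German or English culture.
; Menu and loading-screen widgets are created once, cached and re-added to the viewport.
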(event `self.ReceiveInit`
  ;[1 1 1] Init culture
  (`self.SetCulture` (`self.defaultLanguage`)))

(event `BeginDisasterEventLevelsFromQuiz`
  (params (disasterEvent :type Name))
  ;[1 1 1] Begin playing disasterLevels for specific event
  (bind _output_get (set `self.currentDisasterEvent` disasterEvent))
  (set `self.currentEventLevelNr` 1)
  (bind _returnvalue (`|GetDataTableRow` "/Game/Gameplay/Data/Quiz/disasterEventLevels.disasterEventLevels" _output_get)
    (:`then`
      (`self.EnterDisasterLevel` (`.level01_5_9D3D9EDB4D97166F241DD48736F6EE7E` (break `/Game/Gameplay/Data/Quiz/disasterEventLevelsStruct` _returnvalue))))
    (:`RowNotFound`
      (`/Game/Gameplay/Blueprints/libraries/fonLib.PrintError` "fonInstance BeginDisasterEventLevelsFromQuiz didn't find Row!"))))

(event `PlayDisasterPrototype`
  ;[1 1 1] Play disasterlevel prototype
  (`self.ShowLoadingScreen`)
  (`self.EnterDisasterLevel` "Flood_Cologne_02"))

(event `PlayWorldMapPrototype`
  ;[1 1 1] Play worldmap
  (`self.ShowLoadingScreen`)
  (`GameplayStatics.OpenLevel` "/Game/Levels/worldMapLevels/worldMap"))

(event `PlayMainMenu`
  ;[1 1 1] Return to Main Menu Level (and show main menu
  (`self.ShowLoadingScreen`)
  (`GameplayStatics.OpenLevel` "/Game/Levels/MetaLevels/mainMenu")
  (`self.ShowMainMenu`))

(event `ShowLoadingScreen`
  ;[1 1 1] Shows loading screen
  (`/Engine/EditorBlueprintResources/StandardMacros.IsValid` (`self.loadingScreenWidget`)
    (:`Is Valid`
      _)
    (:`Is Not Valid`
      (bind _returnvalue (`|CreateWidget` "/Game/Gameplay/Blueprints/gui/Menus/LoadingScreen.LoadingScreen_C" (`GameplayStatics.GetPlayerController` 0)))
      (set `self.loadingScreenWidget` _returnvalue)))
  (`UserWidget.AddToViewport` (`self.loadingScreenWidget`) 0))

(event `RemoveLoadingScreen`
  ;[1 1 1] Remove LoadingScreen
  (`/Engine/EditorBlueprintResources/StandardMacros.IsValid` (`self.loadingScreenWidget`)
    (:`Is Valid`
      (`Widget.RemoveFromParent` (`self.loadingScreenWidget`)))))

(event `ShowMainMenu`
  (bind _returnvalue (`GameplayStatics.GetPlayerController` 0))
  ;[1 1 1] Show Main Menu
  (`/Engine/EditorBlueprintResources/StandardMacros.IsValid` (`self.mainMenuWidget`)
    (:`Is Valid`
      _)
    (:`Is Not Valid`
      (bind _returnvalue_2 (`|CreateWidget` "/Game/Gameplay/Blueprints/gui/Menus/MainMenuWidgetNew.MainMenuWidgetNew_C" _returnvalue))
      (set `self.mainMenuWidget` _returnvalue_2)))
  (`UserWidget.AddToViewport` (`self.mainMenuWidget`) 0)
  (set `PlayerController.bShowMouseCursor` true _returnvalue))

(event `ShowOptionsMenu`
  ;[1 1 1] Show Options Menu
  (`/Engine/EditorBlueprintResources/StandardMacros.IsValid` (`self.optionsWidget`)
    (:`Is Valid`
      _)
    (:`Is Not Valid`
      (bind _returnvalue (`|CreateWidget` "/Game/Gameplay/Blueprints/gui/Menus/OptionsMenu.OptionsMenu_C" (`GameplayStatics.GetPlayerController` 0)))
      (set `self.optionsWidget` _returnvalue)))
  (`UserWidget.AddToViewport` (`self.optionsWidget`) 0))

(event `ShowLanguageMenu`
  ;[1 1 1] Show Language Menu
  (`/Engine/EditorBlueprintResources/StandardMacros.IsValid` (`self.languageWidget`)
    (:`Is Valid`
      _)
    (:`Is Not Valid`
      (bind _returnvalue (`|CreateWidget` "/Game/Gameplay/Blueprints/gui/Menus/LanguageMenu.LanguageMenu_C" (`GameplayStatics.GetPlayerController` 0)))
      (set `self.languageWidget` _returnvalue)))
  (`UserWidget.AddToViewport` (`self.languageWidget`) 0))

(event `ShowDebugLevelSelect`
  ;[1 1 1] Show ShowDebugLevelSelect Menu
  (`/Engine/EditorBlueprintResources/StandardMacros.IsValid` (`self.debugLevelSelectWidget`)
    (:`Is Valid`
      _)
    (:`Is Not Valid`
      (bind _returnvalue (`|CreateWidget` "/Game/Gameplay/Blueprints/gui/Menus/DebugLevelSelectMenu.DebugLevelSelectMenu_C" (`GameplayStatics.GetPlayerController` 0)))
      (set `self.debugLevelSelectWidget` _returnvalue)))
  (`UserWidget.AddToViewport` (`self.debugLevelSelectWidget`) 0))

(event `ShowDeveloperOptions`
  ;[1 1 1] Show ShowDebugLevelSelect Menu
  (`/Engine/EditorBlueprintResources/StandardMacros.IsValid` (`self.developerWidget`)
    (:`Is Valid`
      _)
    (:`Is Not Valid`
      (bind _returnvalue (`|CreateWidget` "/Game/Gameplay/Blueprints/gui/Menus/DeveloperMenu.DeveloperMenu_C" (`GameplayStatics.GetPlayerController` 0)))
      (set `self.developerWidget` _returnvalue)))
  (`UserWidget.AddToViewport` (`self.developerWidget`) 0))

(fn `EnterDisasterLevel`
  (params (levelName :type Name))
  (`GameplayStatics.OpenLevel` (`KismetStringLibrary.Conv_StringToName` (`KismetStringLibrary.Concat_StrStr` "/Game/Levels/DisasterLevels/" (`KismetStringLibrary.Conv_NameToString` levelName)))))

(fn `LoadNextLevelInEvent`
  (locals (levelToEnter :type Name))
  (`self.ResetLevelSpecificData`)
  (`/Engine/EditorBlueprintResources/StandardMacros.IncrementInt` (`self.currentEventLevelNr`)
    (:`  `
      (bind _returnvalue (`|GetDataTableRow` "/Game/Gameplay/Data/Quiz/disasterEventLevels.disasterEventLevels" (`self.currentDisasterEvent`))
        (:`then`
          (`|ExecutionSequence`
            (:`then_0`
              ;[1 0 0] Sequence
              (switch `int` (`self.currentEventLevelNr`)
                (:`Default`
                  (`/Game/Gameplay/Blueprints/libraries/fonLib.PrintError` "fonInstance LoadNextLevelInEvent current level number too high!!")
                  (return))
                (:`1`
                  (bind (_level01 _level02 _level03 _level04 _level05 _level06 _level07 _level08 _level09 _level10) (break `/Game/Gameplay/Data/Quiz/disasterEventLevelsStruct` _returnvalue))
                  (set `local.levelToEnter` _level01))
                (:`2`
                  (set `local.levelToEnter` _level02))
                (:`3`
                  (set `local.levelToEnter` _level03))
                (:`4`
                  (set `local.levelToEnter` _level04))
                (:`5`
                  (set `local.levelToEnter` _level05))
                (:`6`
                  (set `local.levelToEnter` _level06))
                (:`7`
                  (set `local.levelToEnter` _level07))
                (:`8`
                  (set `local.levelToEnter` _level08))
                (:`9`
                  (set `local.levelToEnter` _level09))
                (:`10`
                  (set `local.levelToEnter` _level10))))
            (:`then_1`
              (if (== (`local.levelToEnter`) "None")
                (`self.PlayWorldMapPrototype`)
                (else
                  (`self.EnterDisasterLevel` (`local.levelToEnter`)))))))
        (:`RowNotFound`
          (`/Game/Gameplay/Blueprints/libraries/fonLib.PrintError` "fonInstance BeginDisasterEventLevelsFromQuiz didn't find Row!"))))))

(fn `ResetLevelSpecificData`
  (set `self.currentLevelPlayerDeaths` 0)
  (set `self.playerWasKilledByBox3_4` false)
  (set `self.retryingLevel` false))

(fn `RestartDisasterLevel`
  (set `self.retryingLevel` true)
  (bind _returnvalue (`GameplayStatics.GetCurrentLevelName` true))
  (`self.EnterDisasterLevel` (`KismetStringLibrary.Conv_StringToName` _returnvalue)))

(fn `SetCulture`
  (params (Culture :type String))
  (if (`KismetStringLibrary.EqualEqual_StrStr` Culture "de-DE")
    (`KismetInternationalizationLibrary.SetCurrentCulture` Culture true)
    (set `self.languageIsEnglish` false)
    (else
      (`KismetInternationalizationLibrary.SetCurrentCulture` "en" true)
      (set `self.languageIsEnglish` true))))