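; fonLib is a small Blueprint function library of shared gameplay helpers for debug printing and direction math.
; PrintError and PrintInfo wrap PrintString and stay silent when the fonInstance game instance has presentation mode on, with info messages shown in green for longer.
; If the game instance cast fails, both print a failure message instead.
; GetOppositeDirection maps each direction enum value to its opposite, leaving None unchanged.
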(fn `GetOppositeDirection`
  (params (direction :type "/Game/Gameplay/Blueprints/libraries/direction Enum" :default "NewEnumerator4"))
  (returns (oppositeDirection :type "/Game/Gameplay/Blueprints/libraries/direction Enum"))
  (switch `/Game/Gameplay/Blueprints/libraries/direction` direction
    (:`NewEnumerator4`
      (return "NewEnumerator4"))
    (:`NewEnumerator0`
      (return "NewEnumerator2"))
    (:`NewEnumerator1`
      (return "NewEnumerator3"))
    (:`NewEnumerator2`
      (return "NewEnumerator0"))
    (:`NewEnumerator3`
      (return "NewEnumerator1"))))

(fn `PrintError`
  (params (string :type String))
  ;[1 1 1] Do not print stuff in presentation mode!
  (bind _asfon_instance (cast `/Game/Gameplay/Blueprints/core/fonInstance` (`GameplayStatics.GetGameInstance` null))
    (:`then`
      (if (not (`/Game/Gameplay/Blueprints/core/fonInstance.presentationModeOn` _asfon_instance))
        (`KismetSystemLibrary.PrintString` null string true true (struct :`R` 1.0 :`A` 1.0) 60.0)))
    (:`CastFailed`
      (`KismetSystemLibrary.PrintString` null "fonLib PrintError cast to fonInstance failed" true true (struct :`R` 1.0 :`A` 1.0) 30.0))))

(fn `PrintInfo`
  (params (String :type String))
  ;[1 1 1] Do not print stuff in presentation mode!
  (bind _asfon_instance (cast `/Game/Gameplay/Blueprints/core/fonInstance` (`GameplayStatics.GetGameInstance` null))
    (:`then`
      (if (not (`/Game/Gameplay/Blueprints/core/fonInstance.presentationModeOn` _asfon_instance))
        (`KismetSystemLibrary.PrintString` null String true true (struct :`R` 0.280457 :`G` 1.0 :`A` 1.0) 15.0)))
    (:`CastFailed`
      (`KismetSystemLibrary.PrintString` null "fonLib PrintInfo cast to fonInstance failed" true true (struct :`R` 1.0 :`A` 1.0) 30.0))))